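; First-person character Blueprint whose only active logic updates the HUD highlight when the selected tool index changes.
; UIToolIndexSelected gets player 0's HUD as PlayerHUDBP and looks up ToolIconWidgets by index in the HUD widget's ToolBox.
; It clears Selected on the previous icon, then sets it on the new one, stopping early if any cast fails.
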(event `self.UIToolIndexSelected`
  (params (PreviousIndex :type Integer) (NewIndex :type Integer))
  (bind _asplayer_hudbp (cast `/Game/Blueprints/Core/PlayerHUDBP` (`PlayerController.GetHUD` (`GameplayStatics.GetPlayerController` 0))))
  (bind _toolbox (`/Game/Blueprints/UI/HUDWidget.ToolBox` (`/Game/Blueprints/Core/PlayerHUDBP.HUDWidget` _asplayer_hudbp)))
  (bind _astool_icon_widget (cast `/Game/Blueprints/UI/ToolIconWidget` (`PanelWidget.GetChildAt` _toolbox PreviousIndex)))
  (set `/Game/Blueprints/UI/ToolIconWidget.Selected` false _astool_icon_widget)
  (bind _astool_icon_widget_2 (cast `/Game/Blueprints/UI/ToolIconWidget` (`PanelWidget.GetChildAt` _toolbox NewIndex)))
  (set `/Game/Blueprints/UI/ToolIconWidget.Selected` true _astool_icon_widget_2))

(fn `UserConstructionScript`)