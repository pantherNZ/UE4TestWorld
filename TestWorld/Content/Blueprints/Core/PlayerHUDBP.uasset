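; Player HUD Blueprint that creates the main HUD widget on BeginPlay and fills its toolbox with the player's tools.
; It walks the FPCharacter capsule's child components in reverse, giving each BasePlayerTool's name and a wrapped, one-based slot index to the next ToolIconWidget.
; Toolbox slots left without a tool are hidden and tinted nearly transparent.
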(event `self.ReceiveBeginPlay`
  (bind _returnvalue (`GameplayStatics.GetPlayerController` 0))
  (bind _numtools (`self.NumTools`))
  (bind _returnvalue_2 (`|CreateWidget` "/Game/Blueprints/UI/HUDWidget.HUDWidget_C" _returnvalue))
  (`UserWidget.AddToViewport` _returnvalue_2 0)
  (set `self.HUDWidget` _returnvalue_2)
  (bind _asfpcharacter (cast `/Game/Blueprints/Core/FPCharacter` (`GameplayStatics.GetPlayerCharacter` 0)))
  (bind _asplayer_hudbp (cast `/Game/Blueprints/Core/PlayerHUDBP` (`PlayerController.GetHUD` _returnvalue)))
  (bind (_arrayindex _arrayelement) (`/Engine/EditorBlueprintResources/StandardMacros.ReverseForEachLoop` (`SceneComponent.GetChildrenComponents` (`Character.CapsuleComponent` _asfpcharacter) false))
    (:`LoopBody`
      (bind _asbase_player_tool (cast `BasePlayerTool` _arrayelement))
      (bind _toolbox (`/Game/Blueprints/UI/HUDWidget.ToolBox` (`/Game/Blueprints/Core/PlayerHUDBP.HUDWidget` _asplayer_hudbp)))
      (bind _astool_icon_widget (cast `/Game/Blueprints/UI/ToolIconWidget` (`PanelWidget.GetChildAt` _toolbox _numtools)))
      (set `/Game/Blueprints/UI/ToolIconWidget.ToolNameText` (`KismetTextLibrary.Conv_StringToText` (`BasePlayerTool.GetName` _asbase_player_tool)) _astool_icon_widget)
      (bind _returnvalue_3 (`PanelWidget.GetChildrenCount` _toolbox))
      (set `/Game/Blueprints/UI/ToolIconWidget.Index` (mod (+ _numtools 1) _returnvalue_3) _astool_icon_widget)
      (`/Engine/EditorBlueprintResources/StandardMacros.IncrementInt` _numtools))
    (:`Completed`
      (for _index (range _numtools _returnvalue_3)
        (bind _returnvalue_4 (`PanelWidget.GetChildAt` _toolbox _index))
        (bind _astool_icon_widget_2 (cast `/Game/Blueprints/UI/ToolIconWidget` _returnvalue_4))
        (`Widget.SetVisibility` _returnvalue_4 "Hidden")
        (`Widget.SetVisibility` _astool_icon_widget_2 "Hidden")
        (`UserWidget.SetColorAndOpacity` _astool_icon_widget_2 (struct :`A` 0.016))))))

(fn `UserConstructionScript`)